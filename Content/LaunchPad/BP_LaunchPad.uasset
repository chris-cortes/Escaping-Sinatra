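; Launch pad Blueprint that collects deposited resources toward a game win condition.
; DepositResource switches on the resource type, incrementing the stored Aluminum, Oxygen or Hydrogen count and printing it.
; After each deposit it checks all three counts against their required amounts and prints a win message when met.
; EndGame is an empty stub, so winning is only reported through debug prints.
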(event EventBeginPlay)

(event Collision|EventActorBeginOverlap
  (params (OtherActor :type Actor%20Object%20Reference)))

(event EventTick
  (params (DeltaSeconds :type Float%20%28single-precision%29)))

(fn ConstructionScript)

(fn DepositResource
  (params (Resource :type EResources%20Enum :default "NewEnumerator3"))
  (Development|PrintString "Hello")
  (switch Utilities|FlowControl|Switch|SwitchonEResources Resource
    (:NewEnumerator0
      (bind _result (Math|Integer|IncrementInt (Variables|Default|GetStoredAluminum))
        (:%20%20
          (Development|PrintString (Utilities|String|Append "Aluminum: " (Utilities|String|ToString(Integer) _result))))))
    (:NewEnumerator1
      (bind _result_2 (Math|Integer|IncrementInt (Variables|Default|GetStoredOxygen))
        (:%20%20
          (Development|PrintString (Utilities|String|Append "Oxygen: " (Utilities|String|ToString(Integer) _result_2))))))
    (:NewEnumerator2
      (bind _result_3 (Math|Integer|IncrementInt (Variables|Default|GetStoredHydrogen))
        (:%20%20
          (Development|PrintString (Utilities|String|Append "Hydrogen: " (Utilities|String|ToString(Integer) _result_3)))))))
  (if (Math|Boolean|ANDBoolean (>= (Variables|Default|GetStoredAluminum) (Variables|Default|GetRequiredAluminum)) (>= (Variables|Default|GetStoredOxygen) (Variables|Default|GetRequiredOxygen)) (>= (Variables|Default|GetStoredHydrogen) (Variables|Default|GetRequiredHydrogen)))
    (Development|PrintString "Game Win!!")))

(fn EndGame)